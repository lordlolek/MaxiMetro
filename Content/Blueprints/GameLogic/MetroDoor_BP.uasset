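; MetroDoor_BP is a sliding double door for the metro that opens and closes through Open and Close events.
; BeginPlay caches each panel's relative location, then a timeline lerps Left and Right apart along local Y and reverses to close them.
; The timeline's Finished pin calls CallDoorMoveEnd to signal that the movement has ended.
; An unconnected Delay and FlipFlop toggle between Open and Close is left in the graph.
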(event `self.ReceiveBeginPlay`
  (set `self.LeftDefaultLocation` (`SceneComponent.RelativeLocation` (`self.Left`)))
  (set `self.RightDefaultLocation` (`SceneComponent.RelativeLocation` (`self.Right`))))

(event `Open`
  (bind _rightdefaultlocation (`self.RightDefaultLocation`))
  (bind _leftdefaultlocation (`self.LeftDefaultLocation`))
  (bind (_direction _alpha) (`Timeline|T` :!via `PlayFromStart` :!label _label)
    (:`Update`
      (`SceneComponent.K2_SetRelativeLocation` (`self.Left`) (`KismetMathLibrary.VLerp` _leftdefaultlocation (+ _leftdefaultlocation (0.0 -100.0 0.0)) _alpha) false false)
      (`SceneComponent.K2_SetRelativeLocation` (`self.Right`) (`KismetMathLibrary.VLerp` _rightdefaultlocation (+ _rightdefaultlocation (0.0 100.0 0.0)) _alpha) false false))
    (:`Finished`
      (`self.DoorMoveEnd`))))

(event `Close`
  (goto _label :!via `ReverseFromEnd`))

(fn `UserConstructionScript`)