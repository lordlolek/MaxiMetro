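; MetroController_BP drives a Metro reference through a repeating cycle of riding and stopping.
; Tick accumulates a timer and toggles the OnStop state, calling Metro.Stop when the ride time elapses and Metro.Ride when StopTime elapses.
; On each departure, SetNextParams picks a random duration until the next stop from the PossibleTimeToStop range, while the stop duration comes from StopTime.
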(event `self.ReceiveBeginPlay`)

(event `self.ReceiveTick`
  (params (DeltaSeconds :type "Float (single-precision)"))
  (set `self.Timer` (+ DeltaSeconds (`self.Timer`)))
  (if (`self.OnStop`)
    (if (> (`self.Timer`) (`self.StopTime`))
      (set `self.Timer` 0.0)
      (set `self.OnStop` false)
      (`self.SetNextParams`)
      (`/Game/Blueprints/GameLogic/MetroWagon_BP.Ride` (`self.Metro`)))
    (elif (> (`self.Timer`) (`self.NextTimeToStop`))
      (set `self.Timer` 0.0)
      (set `self.OnStop` true)
      (`/Game/Blueprints/GameLogic/MetroWagon_BP.Stop` (`self.Metro`)))))

(fn `SetNextParams`
  (bind (_possibletimetostop_x _possibletimetostop_y) (`KismetMathLibrary.BreakVector2D` (`self.PossibleTimeToStop`)))
  (set `self.NextTimeToStop` (`KismetMathLibrary.RandomFloatInRange` _possibletimetostop_x _possibletimetostop_y)))

(fn `UserConstructionScript`)