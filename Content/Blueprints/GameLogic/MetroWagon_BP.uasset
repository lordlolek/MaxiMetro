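; Metro wagon Blueprint that switches the ride between moving and stopped states.
; On BeginPlay it caches every MetroDoor_BP in the level and the MetroPlayerCharacter.
; Ride closes the doors and sets Riding, while Stop opens them and clears it.
; While Riding, Tick replays a world camera shake centered on the player's camera; OpenDoors and CloseDoors are empty stubs.
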(event `self.ReceiveBeginPlay`
  (bind _outactors (`GameplayStatics.GetAllActorsOfClass` "/Game/Blueprints/GameLogic/MetroDoor_BP.MetroDoor_BP_C"))
  (set `self.MetroDoors` _outactors)
  (bind _asmetro_player_character (cast `/Game/Blueprints/Player/MetroPlayerCharacter` (`GameplayStatics.GetPlayerCharacter` 0)))
  (set `self.Player` _asmetro_player_character))

(event `self.ReceiveTick`
  (params (DeltaSeconds :type "Float (single-precision)"))
  (if (`self.Riding`)
    (`GameplayStatics.PlayWorldCameraShake` "/Game/Blueprints/Misc/RidingCameraShake.RidingCameraShake_C" (`SceneComponent.K2_GetComponentLocation` (`/Game/Blueprints/Player/MetroPlayerCharacter.Camera` (`self.Player`))) 1000.0 1000.0)))

(event `Ride`
  (`/Game/Blueprints/GameLogic/MetroDoor_BP.Close` (`self.MetroDoors`))
  (set `self.Riding` true))

(event `Stop`
  (`/Game/Blueprints/GameLogic/MetroDoor_BP.Open` (`self.MetroDoors`))
  (set `self.Riding` false))

(event `OpenDoors`)

(event `CloseDoors`)

(fn `UserConstructionScript`)