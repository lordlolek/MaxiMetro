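; Chair Blueprint that tracks whether it is occupied and by whom.
; Interact claims a free chair for the caller and releases an occupied one only when that same caller interacts again.
; IsOccupied, Occupy and Free wrap the Occupied flag, while Interact records the Occupier, which Free leaves set.
; It only manages occupancy state, with no movement, attachment or animation.
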(event `/Game/Blueprints/Interaction/InteractionInterface.Interact`
  (params (Caller :type "Actor Object Reference"))
  (if (`self.IsOccupied`)
    (if (== (`self.Occupier`) Caller)
      (`self.Free`))
    (else
      (`self.Occupy`)
      (set `self.Occupier` Caller))))

(fn `Free`
  (set `self.Occupied` false))

(fn `IsOccupied`
  (returns (Occupied :type Boolean))
  (return (`self.Occupied`)))

(fn `Occupy`
  (set `self.Occupied` true))

(fn `UserConstructionScript`)