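; InteractiveActor_Comp is a component that marks its owning actor as interactive and acts as a hover indicator.
; On BeginPlay it adds the "Interactive" tag to the owner's actor tags without duplicates and hides itself.
; Its Hover and Unhover events show and hide the component, without propagating visibility to children.
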(event `self.ReceiveBeginPlay`
  (bind _returnvalue (`self.GetOwner`))
  (bind _output_get (set `self.Tags` (`Actor.Tags` _returnvalue)))
  (`KismetArrayLibrary.Array_AddUnique` _output_get "Interactive")
  (set `Actor.Tags` (`self.Tags`) _returnvalue)
  (`self.SetVisibility` false))

(event `/Game/Blueprints/Interaction/InteractionInterface.Hover`
  (`self.SetVisibility` true))

(event `/Game/Blueprints/Interaction/InteractionInterface.Unhover`
  (`self.SetVisibility` false))