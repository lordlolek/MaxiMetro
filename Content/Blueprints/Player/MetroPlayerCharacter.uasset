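; MetroPlayerCharacter is a cursor-aimed player character that moves along world axes and interacts with tagged objects.
; Each tick it traces under the mouse, moves a crosshair sprite to the hit point and yaws the player mesh toward it.
; CheckIfCanInteract swaps the crosshair sprite for Interactive-tagged actors within range, and the Interaction input sends them InteractMessage.
; A component-based hover/unhover variant is left unconnected.
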(event `self.ReceiveTick`
  (params (DeltaSeconds :type "Float (single-precision)"))
  (set `self.MouseHitResult` (`PlayerController.GetHitResultUnderCursorByChannel` (`GameplayStatics.GetPlayerController` 0) "TraceTypeQuery1" true))
  (`self.SetCursorPosition`)
  (`self.SetPlayerOrientation`)
  (`self.CheckIfCanInteract`))

(event `InputAction|Interaction`
  (params (Key :type "Key Structure"))
  (:`Pressed`
    (bind (_can _actor) (`self.CheckIfCanInteract`))
    (if _can
      (message `/Game/Blueprints/Interaction/InteractionInterface.Interact` _actor))))

(event `InputAxis|MoveUp`
  (params (AxisValue :type "Float (single-precision)"))
  (`self.AddMovementInput` (1.0 0.0 0.0) AxisValue))

(event `InputAxis|MoveRIght`
  (params (AxisValue :type "Float (single-precision)"))
  (`self.AddMovementInput` (0.0 1.0 0.0) AxisValue))

(fn `CheckIfCanInteract`
  (returns (Can :type Boolean) (Actor :type "Actor Object Reference"))
  (bind _crosshair (`self.CrossHair`))
  (bind (_bblockinghit _binitialoverlap _time _distance _location _impactpoint _normal _impactnormal _physmat _hitactor) (`GameplayStatics.BreakHitResult` (`self.MouseHitResult`)))
  (if _bblockinghit
    (if (and (`self.ActorHasTag` _hitactor "Interactive") (<= (`self.GetDistanceTo` _hitactor) (`self.InteractionRange`)))
      (`BillboardComponent.SetSprite` _crosshair "/Engine/EngineResources/AICON-Green.AICON-Green")
      (return true _hitactor)
      (else
        (`BillboardComponent.SetSprite` _crosshair "/Engine/MobileResources/HUD/AnalogHat.AnalogHat")
        (return false null)))))

(fn `SetCrossHairLocation`
  (`SceneComponent.K2_SetWorldLocation` (`self.CrossHair`) (`self.CursorPostition`) false false))

(fn `SetCursorPosition`
  (set `self.CursorPostition` (`.Location` (`GameplayStatics.BreakHitResult` (`self.MouseHitResult`))))
  (`self.SetCrossHairLocation`))

(fn `SetPlayerOrientation`
  (bind _playermesh (`self.PlayerMesh`))
  (bind (_returnvalue_roll _returnvalue_pitch _returnvalue_yaw) (`KismetMathLibrary.BreakRotator` (`KismetMathLibrary.FindLookAtRotation` (`SceneComponent.K2_GetComponentLocation` _playermesh) (`self.CursorPostition`))))
  (`SceneComponent.K2_SetWorldRotation` _playermesh (`KismetMathLibrary.MakeRotator` 0.0 0.0 _returnvalue_yaw) false false))

(fn `UserConstructionScript`)